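; FastOrNotCharacter is the player character for a timed level, moving along the world X axis and jumping.
; A timeline starts on BeginPlay and serves as the clock, copied into CurrentTime every tick.
; TimeOut and LevelFinished events set a failure or success message, the latter including the time.
; Both then share one path that shows the LevelEndMenu widget, switches to UI-only input with a cursor and stops controller movement.
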(event `self.ReceiveBeginPlay`
  (bind (_direction _currenttimeline) (`Timeline|Timeline_0`)))

(event `self.ReceiveTick`
  (params (DeltaSeconds :type "Float (single-precision)"))
  (set `self.CurrentTime` (stale `self.ReceiveBeginPlay` _currenttimeline)))

(event `self.ReceiveActorBeginOverlap`
  (params (OtherActor :type "Actor Object Reference")))

(event `InputAxis|MoveRight`
  (params (AxisValue :type "Float (single-precision)"))
  (`self.AddMovementInput` (1.0 0.0 0.0) AxisValue))

(event `InputAction|Jump`
  (:`Pressed`
    (`self.Jump`)))

(event `TimeOut`
  (bind _returnvalue (`GameplayStatics.GetPlayerController` 0))
  (set `self.LevelEndText` "Shucks! You ran out of time:(")
  (bind _returnvalue_2 (`|CreateWidget` "/Game/FastOrNotContent/Blueprints/Menus/LevelEndMenu.LevelEndMenu_C" :!label _label))
  (`UserWidget.AddToViewport` _returnvalue_2 0)
  (set `PlayerController.bShowMouseCursor` true _returnvalue)
  (`WidgetBlueprintLibrary.SetInputMode_UIOnlyEx` _returnvalue)
  (`Controller.StopMovement` _returnvalue))

(event `self.ReceiveDestroyed`)

(event `LevelFinished`
  (set `self.LevelEndText` (`KismetTextLibrary.Conv_StringToText` (`KismetStringLibrary.Concat_StrStr` "Hurray! You finished the level with time: " (`KismetStringLibrary.Conv_DoubleToString` (`self.CurrentTime`)))))
  (goto _label))

(fn `UserConstructionScript`)